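; Game mode for the builder game that gives each of two players a different character, Bridge Builder or Tower Builder.
; On PostLogin, it matches the new controller against player index 0 or 1.
; It spawns the matching character at the player start named "Bridge" or "Tower", owned by that controller, and possesses it.
; Any other controller only prints an invalid-controller message.
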(event `self.K2_PostLogin`
  (params (NewPlayer :type "PlayerController Object Reference"))
  (bind _returnvalue (`GameplayStatics.GetPlayerController` 0))
  (bind _returnvalue_2 (`GameplayStatics.GetPlayerController` 1))
  (if (== (`GameplayStatics.GetPlayerController` 0) NewPlayer)
    (bind _returnvalue_3 (`|SpawnActorFromClass` "/Game/ThirdPerson/Blueprints/BP_Char_BridgeBuilder.BP_Char_BridgeBuilder_C" (`self.GetTransform` (`self.K2_FindPlayerStart` _returnvalue "Bridge")) "Undefined" "MultiplyWithRoot" _returnvalue null))
    (`Controller.Possess` (`GameplayStatics.GetPlayerController` 0) _returnvalue_3)
    (elif (== (`GameplayStatics.GetPlayerController` 1) NewPlayer)
      (bind _returnvalue_4 (`|SpawnActorFromClass` "/Game/ThirdPerson/Blueprints/BP_Char_TowerBuilder.BP_Char_TowerBuilder_C" (`self.GetTransform` (`self.K2_FindPlayerStart` _returnvalue_2 "Tower")) "Undefined" "MultiplyWithRoot" _returnvalue_2 null))
      (`Controller.Possess` (`GameplayStatics.GetPlayerController` 1) _returnvalue_4)
      (else
        (`KismetSystemLibrary.PrintString` "Not a valid controller")))))

(fn `UserConstructionScript`)