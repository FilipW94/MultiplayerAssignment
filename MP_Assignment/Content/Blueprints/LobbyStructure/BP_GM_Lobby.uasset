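; Lobby GameMode that registers joining players, spawns their lobby characters and server-travels to the construction site level on launch.
; On post-login, the authority reads server settings from the game instance, initializes the player's lobby controller and possesses a character spawned at a random PlayerStart.
; EveryoneUpdate rebuilds the player list, pushes it to all controllers and sets CanWeStart from character selections.
; Character swap and kick events are empty stubs.
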(event `self.K2_PostLogin`
  (params (NewPlayer :type "PlayerController Object Reference"))
  ; Initial Setup on EventPostLogin - Handles ServerName and Player Spawn
  (`/Engine/EditorBlueprintResources/ActorMacros.Switch Has Authority`
    (:`Authority`
      (`KismetArrayLibrary.Array_Add` (`self.AllPlayerControllers`) NewPlayer)
      (bind _outactors (`GameplayStatics.GetAllActorsOfClass` "/Script/Engine.PlayerStart"))
      (set `self.SpawnPoints` _outactors)
      (bind _asbp_builder_game_instance (cast `/Game/Blueprints/CoreGameStructure/BP_BuilderGameInstance` (`GameplayStatics.GetGameInstance`)))
      (set `self.Max Players` (`/Game/Blueprints/CoreGameStructure/BP_BuilderGameInstance.MaxPlayers` _asbp_builder_game_instance))
      (set `self.Server Name` (`/Game/Blueprints/CoreGameStructure/BP_BuilderGameInstance.ServerName` _asbp_builder_game_instance))
      (bind _asbp_pc_lobby (cast `/Game/Blueprints/LobbyStructure/BP_PC_Lobby` NewPlayer))
      (`/Game/Blueprints/LobbyStructure/BP_PC_Lobby.InitialSetup` _asbp_pc_lobby)
      (`/Game/Blueprints/LobbyStructure/BP_PC_Lobby.SetupLobbyMenu` _asbp_pc_lobby (`self.Server Name`))
      (`self.RespawnPlayer` NewPlayer))))

(event `RespawnPlayer`
  (params (PlayerController :type "PlayerController Object Reference"))
  (bind _returnvalue (`Controller.K2_GetPawn` PlayerController))
  (bind _spawnpoints (`self.SpawnPoints`))
  ; Spawn player as lobby character when arriving at the lobby menu - Tells every Player to update their lobby
  (`/Engine/EditorBlueprintResources/StandardMacros.IsValid` _returnvalue
    (:`Is Valid`
      (`self.K2_DestroyActor` _returnvalue))
    (:`Is Not Valid`
      _))
  (bind _returnvalue_2 (`|SpawnActorFromClass` "/Game/Blueprints/ServerSelectStructure/BP_LobbyCharacter.BP_LobbyCharacter_C" (`self.GetTransform` (`|GetArrayItem` _spawnpoints (`KismetMathLibrary.RandomIntegerInRange` 0 (- (`KismetArrayLibrary.Array_Length` _spawnpoints) 1)))) "Undefined" "MultiplyWithRoot" null null))
  (`Controller.Possess` PlayerController _returnvalue_2)
  (`self.EveryoneUpdate`))

(event `LaunchTheGame`
  (`KismetSystemLibrary.ExecuteConsoleCommand` "servertravel /Game/Levels/LVL_ConstructionSite" (`GameplayStatics.GetPlayerController` 0)))

(event `EveryoneUpdate`
  (bind _allplayercontrollers (`self.AllPlayerControllers`))
  (bind _output_get (set `self.CurrentPlayers` (`KismetArrayLibrary.Array_Length` (`self.AllPlayerControllers`))))
  (if (> _output_get 0)
    (`KismetArrayLibrary.Array_Clear` (`self.ConnectedPlayers`))
    (for _array_element _allplayercontrollers
      (bind _asbp_pc_lobby (cast `/Game/Blueprints/LobbyStructure/BP_PC_Lobby` _array_element))
      (`KismetArrayLibrary.Array_Add` (`self.ConnectedPlayers`) (`/Game/Blueprints/LobbyStructure/BP_PC_Lobby.PlayerInfo` _asbp_pc_lobby))
      (`/Game/Blueprints/LobbyStructure/BP_PC_Lobby.UpdateNumberOfPlayers` _asbp_pc_lobby (`self.CurrentPlayers`) (`self.Max Players`)))
    (for _array_element_2 _allplayercontrollers
      (bind _asbp_pc_lobby_2 (cast `/Game/Blueprints/LobbyStructure/BP_PC_Lobby` _array_element_2))
      (`/Game/Blueprints/LobbyStructure/BP_PC_Lobby.AddPlayerInfo` _asbp_pc_lobby_2 (`self.ConnectedPlayers`))
      (`/Game/Blueprints/LobbyStructure/BP_PC_Lobby.UpdateAvailableCharacters` _asbp_pc_lobby_2 (`self.Available Characters`)))
    (for _array_element_3 (`self.ConnectedPlayers`) :!label _label
      (if (== (`.CharacterType_8_8A770B514AA1D26C7978D6BB14DC9BB1` (break `/Game/Blueprints/Structs/F_PlayerInfo` _array_element_3)) 0)
        (set `self.CanWeStart` false)
        (`self.CannotStartGame`)
        (else
          (set `self.CanWeStart` true))))))

(event `CannotStartGame`
  (goto _label :!via `Break`))

(event `SwapCharacter`
  (params (PlayerController :type "PlayerController Object Reference") (CharacterType :type "/Game/Blueprints/Enums/E_CharacterType Enum" :default "NewEnumerator2") (ChangedStatus :type Boolean)))

(event `AddToKickList`)

(fn `UserConstructionScript`)