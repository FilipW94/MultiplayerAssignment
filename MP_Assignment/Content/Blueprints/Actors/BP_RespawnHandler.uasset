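; BP_RespawnHandler tracks the current closest spawn point for the Bridge Builder and Tower Builder characters and supplies it for respawning.
; Shortly after BeginPlay it gathers all BP_SpawnPoint actors, sorts them by character and binds to each one's closest-spawn-detected event.
; When a point reports in, the handler moves that character's ClosestSpawn flag to it.
; GetClosestSpawn returns the stored point's SpawnPoint for the requested character.
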(event `self.ReceiveBeginPlay`
  (`KismetSystemLibrary.Delay` 0.2)
  (`self.SortSpawns`))

(event `SortSpawns`
  (bind _outactors (`GameplayStatics.GetAllActorsOfClass` "/Game/Blueprints/Actors/BP_SpawnPoint.BP_SpawnPoint_C"))
  (for _array_element _outactors
    (switch `/Game/Blueprints/Enums/E_CharacterType` (`/Game/Blueprints/Actors/BP_SpawnPoint.CharacterSpawn` _array_element)
      (:`NewEnumerator0`
        (`KismetArrayLibrary.Array_Add` (`self.BridgeBuilderSpawns`) _array_element))
      (:`NewEnumerator1`
        (`KismetArrayLibrary.Array_Add` (`self.TowerBuilderSpawns`) _array_element))))
  (`self.SetBridgeSpawnListeners`))

(event `SetBridgeSpawnListeners`
  (for _array_element (`self.BridgeBuilderSpawns`)
    (add `/Game/Blueprints/Actors/BP_SpawnPoint.NewClosestSpawnDetected` _array_element (delegate `NewClosestBridgeSpawn`)))
  (`self.SetTowerSpawnListeners`))

(event `NewClosestBridgeSpawn`
  (params (NewClosestSpawn :type "/Game/Blueprints/Actors/BP_SpawnPoint Object Reference"))
  (bind _closestbridgebuilderspawn (`self.ClosestBridgeBuilderSpawn`))
  (`/Engine/EditorBlueprintResources/StandardMacros.IsValid` _closestbridgebuilderspawn
    (:`Is Valid`
      (set `/Game/Blueprints/Actors/BP_SpawnPoint.ClosestSpawn` false _closestbridgebuilderspawn))
    (:`Is Not Valid`
      _))
  (bind _output_get (set `self.ClosestBridgeBuilderSpawn` NewClosestSpawn))
  (set `/Game/Blueprints/Actors/BP_SpawnPoint.ClosestSpawn` true _output_get))

(event `SetTowerSpawnListeners`
  (for _array_element (`self.TowerBuilderSpawns`)
    (add `/Game/Blueprints/Actors/BP_SpawnPoint.NewClosestSpawnDetected` _array_element (delegate `NewClosestTowerSpawn`))))

(event `NewClosestTowerSpawn`
  (params (NewClosestSpawn :type "/Game/Blueprints/Actors/BP_SpawnPoint Object Reference"))
  (bind _closesttowerbuilderspawn (`self.ClosestTowerBuilderSpawn`))
  (`/Engine/EditorBlueprintResources/StandardMacros.IsValid` _closesttowerbuilderspawn
    (:`Is Valid`
      (set `/Game/Blueprints/Actors/BP_SpawnPoint.ClosestSpawn` false _closesttowerbuilderspawn))
    (:`Is Not Valid`
      _))
  (bind _output_get (set `self.ClosestTowerBuilderSpawn` NewClosestSpawn))
  (set `/Game/Blueprints/Actors/BP_SpawnPoint.ClosestSpawn` true _output_get))

(fn `GetClosestSpawn`
  (params (CharacterToSpawn :type "/Game/Blueprints/Enums/E_CharacterType Enum" :default "NewEnumerator2"))
  (returns (SpawnLocation :type "PlayerStart Object Reference"))
  (switch `/Game/Blueprints/Enums/E_CharacterType` CharacterToSpawn
    (:`NewEnumerator0`
      (return (`/Game/Blueprints/Actors/BP_SpawnPoint.SpawnPoint` (`self.ClosestBridgeBuilderSpawn`))))
    (:`NewEnumerator1`
      (return (`/Game/Blueprints/Actors/BP_SpawnPoint.SpawnPoint` (`self.ClosestTowerBuilderSpawn`))))))

(fn `UserConstructionScript`)