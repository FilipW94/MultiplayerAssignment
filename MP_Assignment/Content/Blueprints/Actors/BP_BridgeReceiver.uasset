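; Interactable bridge receiver that builds a bridge step by step while the correct character type holds Interact, and retracts it afterwards.
; On BeginPlay, a forward line trace sets the end point, the spline fills with evenly spaced points, and a BP_BridgeStep spawns at each.
; Tick, enabled on demand, converts rising or falling HoldDuration into a step index to construct or destruct steps.
; A testing timer delays retraction after release.
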(event `DelayBridgeDestruct`
  ; To allow testing. Would required another person to hold interact for bridge to stay up otherwise
  (set `self.DestructTimerActive` true)
  (`KismetSystemLibrary.K2_SetTimerDelegate` (delegate `StopDestructDelay`) 5.0))

(event `StopDestructDelay`
  ; To allow testing. Would required another person to hold interact for bridge to stay up otherwise
  (set `self.DestructTimerActive` false))

(event `self.ReceiveBeginPlay`
  (`SplineComponent.ClearSplinePoints` (`self.BridgeSpline`) true)
  (`self.FindBridgeEnd`)
  (`self.CreateSplineOpposites`))

(event `DestructBridge`
  (bind _returnvalue (`KismetMathLibrary.Clamp` (`KismetMathLibrary.Round` (* (`self.HoldDuration`) 10.0)) 0 (`self.StepsNeeded`)))
  (if (not (>= _returnvalue (`self.PreviousIndex`)))
    (`/Game/Blueprints/Actors/BP_BridgeStep.DestructStep` (`|GetArrayItem` (`self.StepArray`) (`self.PreviousIndex`)))
    (set `self.PreviousIndex` _returnvalue)))

(event `ConstructBridge`
  (bind _returnvalue (`KismetMathLibrary.Clamp` (`KismetMathLibrary.Round` (* (`self.HoldDuration`) 10.0)) 0 (`self.StepsNeeded`)))
  (if (not (<= _returnvalue (`self.PreviousIndex`)))
    (`/Game/Blueprints/Actors/BP_BridgeStep.ConstructStep` (`|GetArrayItem` (`self.StepArray`) (`self.PreviousIndex`)))
    (set `self.PreviousIndex` _returnvalue)))

(event `self.ReceiveTick`
  (params (DeltaSeconds :type "Float (single-precision)"))
  (if (`self.InteractInProgress`)
    ; Increase HoldDuration if Interacted with
    (set `self.HoldDuration` (+ (`self.HoldDuration`) DeltaSeconds))
    (`self.ConstructBridge`)
    (elif (<= (`self.HoldDuration`) 0.0)
      ; Disable Tick if HoldDuration is reduced to 0
      (bind _output_get (set `self.HoldDuration` 0.0))
      (`KismetSystemLibrary.PrintString` (`KismetStringLibrary.Conv_DoubleToString` _output_get) true true (struct :`G` 0.66 :`B` 1.0 :`A` 1.0) 0.1)
      (`self.SetActorTickEnabled` false)
      (bind _output_get_2 (set `self.PreviousIndex` 0))
      (`/Game/Blueprints/Actors/BP_BridgeStep.DestructStep` (`|GetArrayItem` (`self.StepArray`) _output_get_2))
      (else
        ; Decrease HoldDuration if not Interacted with
        (if (not (`self.DestructTimerActive`))
          (bind _output_get_3 (set `self.HoldDuration` (- (`self.HoldDuration`) DeltaSeconds)))
          (`self.DestructBridge`))))))

(event `CreateSplineOpposites`
  (`SplineComponent.AddSplinePoint` (`self.BridgeSpline`) (`SceneComponent.K2_GetComponentLocation` (`self.ReceiverCenter`)) "World" true)
  (`SplineComponent.AddSplinePoint` (`self.BridgeSpline`) (`self.BridgeEndPoint`) "World" true)
  (`self.FillSpline`))

(event `FillSpline`
  (`self.GetStepRequired`)
  (for _index (range (+ (`self.StepsNeeded`) 1))
    (`SplineComponent.AddSplinePoint` (`self.BridgeSpline`) (`self.FindPointCloserToSplineEnd` (* _index (`self.BridgeStepDistance`))) "World" false))
  (`SplineComponent.RemoveSplinePoint` (`self.BridgeSpline`) 1 true)
  (`self.AddSteps`))

(event `AddSteps`
  (for _index (range (`SplineComponent.GetNumberOfSplinePoints` (`self.BridgeSpline`)))
    (bind (_returnvalue_location _returnvalue_rotation) (`KismetMathLibrary.BreakTransform` (`SplineComponent.GetTransformAtSplinePoint` (`self.BridgeSpline`) _index "World" false)))
    (bind _returnvalue (`|SpawnActorFromClass` "/Game/Blueprints/Actors/BP_BridgeStep.BP_BridgeStep_C" (`KismetMathLibrary.MakeTransform` _returnvalue_location _returnvalue_rotation) "Undefined" "MultiplyWithRoot" null null))
    (`KismetArrayLibrary.Array_Add` (`self.StepArray`) _returnvalue))
  (set `self.RequiredHoldDuration` (* (`self.StepsNeeded`) (`self.EachStepHoldDuration`))))

(fn `FindBridgeEnd`
  (bind _receivercenter (`self.ReceiverCenter`))
  (bind _returnvalue (`SceneComponent.K2_GetComponentLocation` _receivercenter))
  (bind _outhit (`KismetSystemLibrary.LineTraceSingle` :`Start` _returnvalue :`End` (+ _returnvalue (* (`SceneComponent.GetForwardVector` _receivercenter) (`self.TraceDistance`))) :`TraceChannel` "TraceTypeQuery1" :`DrawDebugType` "ForDuration"))
  (if (`GameplayStatics.BreakHitResult` _outhit)
    (bind _output_get (set `self.BridgeEndPoint` (`.Location` (`GameplayStatics.BreakHitResult` _outhit))))
    (set `self.BridgeDesiredLength` (`KismetMathLibrary.Vector_Distance` (`SceneComponent.K2_GetComponentLocation` (`self.ReceiverCenter`)) _output_get))
    (else
      (bind _output_get_2 (set `self.BridgeEndPoint` (`.TraceEnd` (`GameplayStatics.BreakHitResult` _outhit))))
      (set `self.BridgeDesiredLength` (`KismetMathLibrary.Vector_Distance` (`SceneComponent.K2_GetComponentLocation` (`self.ReceiverCenter`)) _output_get_2)))))

(fn `FindPointCloserToSplineEnd`
  (params (StepDistance :type "Float (double-precision)"))
  (returns (PointCloserToSplineEnd :type "Vector Structure"))
  (return (+ (`SplineComponent.GetLocationAtSplinePoint` (`self.BridgeSpline`) 0 "World") (* (`self.GetSplineDirection`) StepDistance))))

(fn `GetSplineDirection`
  (returns (DirectionVector :type "Vector Structure"))
  (return (`KismetMathLibrary.Normal` (- (`SplineComponent.GetLocationAtSplinePoint` (`self.BridgeSpline`) 1 "World") (`SplineComponent.GetLocationAtSplinePoint` (`self.BridgeSpline`) 0 "World")))))

(fn `GetStepRequired`
  (set `self.StepsNeeded` (+ (`KismetMathLibrary.Round` (/ (`self.BridgeDesiredLength`) (`self.BridgeStepDistance`))) 1))
  (return))

(fn `Interact`
  (params (PlayerState :type "PlayerState Object Reference") (CharacterType :type "/Game/Blueprints/Enums/E_CharacterType Enum" :default "NewEnumerator2") (InteractInProgress :type Boolean))
  (returns (Success :type Boolean))
  ; Make sure the correct character is interacting
  (if (`|EnumEquality` CharacterType "NewEnumerator0")
    (bind _output_get (set `self.InteractInProgress` InteractInProgress))
    (if _output_get
      ; Tick handles both increase and decrease to HoldDuration but is disabled when not used so it needs to be enabled
      (if (`self.IsActorTickEnabled`)
        (if (>= (`self.HoldDuration`) (`self.RequiredHoldDuration`))
          (set `self.HoldDuration` (`self.RequiredHoldDuration`))
          (return true)
          (else
            (return true)))
        (else
          (`self.SetActorTickEnabled` true)))
      (else
        (`self.DelayBridgeDestruct`)
        (return false)))
    (else
      (`self.DelayBridgeDestruct`)
      (set `self.InteractInProgress` false)
      (return false))))

(fn `UserConstructionScript`)