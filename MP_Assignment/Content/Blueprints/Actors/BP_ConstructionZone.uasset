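; Construction zone actor that flags when a character of the matching construction type enters or leaves its box trigger.
; Overlap events check the character type through BPI_CharacterData, then send an on/off status through BPI_SetConstructionStatus.
; With authority, only a locally controlled pawn updates its HUD and calls the server status message.
; Remote instances call the character's regular status message without a local-control check.
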(event `self.Box.OnComponentBeginOverlap`
  (params (OverlappedComponent :type "PrimitiveComponent Object Reference") (OtherActor :type "Actor Object Reference") (OtherComp :type "PrimitiveComponent Object Reference") (OtherBodyIndex :type Integer) (bFromSweep :type Boolean) (SweepResult :type "HitResult Structure (by ref)"))
  (bind (_aspawn _bsuccess) (cast `Pawn` OtherActor :!pure true))
  (bind (_asplayer_controller _bsuccess_2) (cast `PlayerController` (`Pawn.GetController` _aspawn) :!pure true))
  (if (`KismetSystemLibrary.DoesImplementInterface` OtherActor "/Game/Blueprints/Interfaces/BPI_CharacterData.BPI_CharacterData_C")
    (bind _charactertype (message `/Game/Blueprints/Interfaces/BPI_CharacterData.GetCharacterData` OtherActor))
    (if (`|EnumEquality` _charactertype (`self.ConstructionType`))
      (if (`KismetSystemLibrary.DoesImplementInterface` OtherActor "/Game/Blueprints/Interfaces/BPI_SetConstructionStatus.BPI_SetConstructionStatus_C")
        (`/Engine/EditorBlueprintResources/ActorMacros.Switch Has Authority`
          (:`Authority`
            (if (and (`Pawn.IsLocallyControlled` _aspawn) _bsuccess _bsuccess_2)
              (message `/Game/Blueprints/Interfaces/BPI_HUDCommunication.SetConstructionZoneStatus` (`PlayerController.GetHUD` _asplayer_controller) true)
              (message `/Game/Blueprints/Interfaces/BPI_SetConstructionStatus.SetServerConstructionStatus` OtherActor true)))
          (:`Remote`
            (message `/Game/Blueprints/Interfaces/BPI_SetConstructionStatus.SetConstructionStatus` OtherActor true)))))))

(event `self.Box.OnComponentEndOverlap`
  (params (OverlappedComponent :type "PrimitiveComponent Object Reference") (OtherActor :type "Actor Object Reference") (OtherComp :type "PrimitiveComponent Object Reference") (OtherBodyIndex :type Integer))
  (bind (_aspawn _bsuccess) (cast `Pawn` OtherActor :!pure true))
  (bind (_asplayer_controller _bsuccess_2) (cast `PlayerController` (`Pawn.GetController` _aspawn) :!pure true))
  (if (`KismetSystemLibrary.DoesImplementInterface` OtherActor "/Game/Blueprints/Interfaces/BPI_CharacterData.BPI_CharacterData_C")
    (bind _charactertype (message `/Game/Blueprints/Interfaces/BPI_CharacterData.GetCharacterData` OtherActor))
    (if (`|EnumEquality` _charactertype (`self.ConstructionType`))
      (if (`KismetSystemLibrary.DoesImplementInterface` OtherActor "/Game/Blueprints/Interfaces/BPI_SetConstructionStatus.BPI_SetConstructionStatus_C")
        (`/Engine/EditorBlueprintResources/ActorMacros.Switch Has Authority`
          (:`Authority`
            (if (and (`Pawn.IsLocallyControlled` _aspawn) _bsuccess _bsuccess_2)
              (message `/Game/Blueprints/Interfaces/BPI_HUDCommunication.SetConstructionZoneStatus` (`PlayerController.GetHUD` _asplayer_controller) false)
              (message `/Game/Blueprints/Interfaces/BPI_SetConstructionStatus.SetServerConstructionStatus` OtherActor false)))
          (:`Remote`
            (message `/Game/Blueprints/Interfaces/BPI_SetConstructionStatus.SetConstructionStatus` OtherActor false)))))))

(fn `UserConstructionScript`)