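; Interactable construction site that raises or removes a spiral-stair tower while one character type interacts or releases.
; On BeginPlay an upward trace sets the height, then splines place spawned BP_TowerPillar and BP_TowerStep actors.
; Replicated InteractInProgress plays or reverses a timeline that toggles pieces by index, catching up any skipped by frame drops.
; A safety capsule follows build progress and flags players, blocking construction when it next starts.
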(event `self.ReceiveBeginPlay`
  (`SplineComponent.ClearSplinePoints` (`self.TowerSpline`) true)
  ; Raycast to find either a blocking hit above the SM_ConstructionSite, in which an offset if added downwards to account for the room the player would need.
  ; If no blocking hit: Grab the end of the raycast without any modification
  (`self.FindTowerTop`)
  (`self.CreateSplineOpposites`))

(event `CreateSplineOpposites`
  ;[0.15 0 0.1179 0.5] Create points at both ends of the spline. Splines are currently part of a scale-up plan and could be replaced by a Vector3 array
  (`SplineComponent.AddSplinePoint` (`self.TowerSpline`) (`SceneComponent.K2_GetComponentLocation` (`self.SM_ConstructionSite`)) "World" true)
  (`SplineComponent.AddSplinePoint` (`self.TowerSpline`) (`self.TowerTopPoint`) "World" true)
  (`self.FillSpline`))

(event `ConstructTower`
  (bind _previousstepindex (`self.PreviousStepIndex`))
  (bind _output (`|GetArrayItem` (`self.TowerStepArray`)))
  (bind _output_2 (`|GetArrayItem` (`self.TowerPillarArray`)))
  (bind _output_3 (`|GetArrayItem` (`self.TowerPillarArray`) (/ _previousstepindex (`self.StepsPerBlock`))))
  (bind _returnvalue (== (mod _previousstepindex (`self.StepsPerBlock`)) 0))
  ; General flow of Constructing and Destructing
  (if (`self.PlayerBlocking`)
    (`KismetSystemLibrary.PrintString` "Player blocking")
    (`self.StopTimeline`)
    (else
      (`KismetSystemLibrary.PrintString` "Player NOT blocking")
      (bind (_direction _alpha) (`Timeline|TL_Construct` :!label _label)
        (:`Update`
          (switch `ETimelineDirection` _direction
            (:`Forward`
              (bind _returnvalue_2 (`KismetMathLibrary.Clamp` (`KismetMathLibrary.Round` (`KismetMathLibrary.Lerp` 0.0 (`KismetMathLibrary.Conv_IntToDouble` (`self.TowerStepsNeeded`)) _alpha)) 0 (`self.TowerStepsNeeded`)))
              ;;[0.1366 0.15 0.009436 0.5] Check to prevent the same index from being called more than once
              (set `self.CurrentStepIndex` _returnvalue_2)
              (if (not (<= _returnvalue_2 (`self.PreviousStepIndex`)))
                (`/Game/Blueprints/Actors/BP_TowerStep.ConstructStep` (`|GetArrayItem` (`self.TowerStepArray`) (`self.PreviousStepIndex`)))
                (if _returnvalue
                  (`/Game/Blueprints/Actors/BP_TowerPillar.ConstructPillar` _output_3))
                ;;[0.15 0.1134 0 0.5] Frame drop might cause indexes to be skipped, this is a security measure that checks if one or more indexes has been skipped
                (if (> (- (`self.CurrentStepIndex`) (`self.PreviousStepIndex`)) 1)
                  (`self.StopTimeline` :!label _label_2)
                  (`self.CheckMissedPieces`)
                  (else
                    (set `self.PreviousStepIndex` (`self.CurrentStepIndex`))
                    (`self.SetSafetyCollision`)))))
            (:`Backward`
              (set `self.CurrentStepIndex` _returnvalue_2)
              (if (not (>= _returnvalue_2 (`self.PreviousStepIndex`)))
                (`/Game/Blueprints/Actors/BP_TowerStep.DestructStep` (`|GetArrayItem` (`self.TowerStepArray`) (`self.PreviousStepIndex`)))
                (if _returnvalue
                  (`/Game/Blueprints/Actors/BP_TowerPillar.DestructPillar` _output_3))
                (if (> (- (`self.PreviousStepIndex`) (`self.CurrentStepIndex`)) 1)
                  (goto _label_2)
                  (else
                    (set `self.PreviousStepIndex` (`self.CurrentStepIndex`))
                    (`self.SetSafetyCollision`)))))))
        (:`Finished`
          ;; Make sure the last pillar and step are disabled
          (switch `ETimelineDirection` _direction
            (:`Backward`
              (if (`/Game/Blueprints/Actors/BP_TowerStep.IsActive` _output)
                (`/Game/Blueprints/Actors/BP_TowerStep.DestructStep` _output)
                (if (`/Game/Blueprints/Actors/BP_TowerPillar.isActive` _output_2)
                  (`/Game/Blueprints/Actors/BP_TowerPillar.DestructPillar` _output_2))))))))))

(event `StopTimeline`
  ; General flow of Constructing and Destructing
  (goto _label :!via `Stop`))

(event `DestructTower`
  ; General flow of Constructing and Destructing
  (goto _label :!via `Reverse`))

(event `FillSpline`
  ;[0.15 0 0.09217 0.5] Add point to the spline inbetween the points created above.
  ; Amount of point is dependent on the raycast.
  ; Distance between points is hard-set to align with the size of the pillars
  (`self.GetStepsRequired`)
  (for _index (range 1 (+ (`self.TowerBlocksNeeded`) 1))
    (`SplineComponent.AddSplinePoint` (`self.TowerSpline`) (`self.FindPointCloserToSplineEnd` (* _index (`self.TowerBlockHeight`))) "World" false))
  (`SplineComponent.RemoveSplinePoint` (`self.TowerSpline`) 1 true)
  (`self.AddPillars`))

(event `AddPillars`
  ;[0.01344 0 0.15 0.5] Spawning the pillars used in the tower at their designated location and adding them to an array
  (for _index (range (`SplineComponent.GetNumberOfSplinePoints` (`self.TowerSpline`)))
    (bind _returnvalue_location (`KismetMathLibrary.BreakTransform` (`SplineComponent.GetTransformAtSplinePoint` (`self.TowerSpline`) _index "World" false)))
    (bind _returnvalue (`|SpawnActorFromClass` "/Game/Blueprints/Actors/BP_TowerPillar.BP_TowerPillar_C" (`KismetMathLibrary.MakeTransform` _returnvalue_location) "Undefined" "MultiplyWithRoot" null null))
    (`KismetArrayLibrary.Array_Add` (`self.TowerPillarArray`) _returnvalue))
  ; Actual spaghetti. Pretty much just finding points from a start position with an incremental Z-axis offset and Yaw rotational offset to create a spiral stair
  (`self.FindEachStepLocation`))

(event `CheckMissedPieces`
  (if (`self.InteractInProgress`)
    ;[0.15 0 0 0.5] Construct pieces that was missed due to frame drop
    (for _index (range (`self.PreviousStepIndex`) (+ (`self.CurrentStepIndex`) 1))
      (bind _output (`|GetArrayItem` (`self.TowerStepArray`) _index))
      (if (not (`/Game/Blueprints/Actors/BP_TowerStep.IsActive` _output))
        (`/Game/Blueprints/Actors/BP_TowerStep.ConstructStep` _output)
        (if (== (mod _index (`self.StepsPerBlock`)) 0)
          (bind _output_2 (`|GetArrayItem` (`self.TowerPillarArray`) (/ _index 5)))
          (if (not (`/Game/Blueprints/Actors/BP_TowerPillar.isActive` _output_2))
            (`/Game/Blueprints/Actors/BP_TowerPillar.ConstructPillar` _output_2)))))
    (set `self.PreviousStepIndex` (`self.CurrentStepIndex`))
    (`self.ConstructTower`)
    (else
      ;[0.15 0 0 0.5] Destruct pieces that were missed cause of frame drop
      (for _index_2 (range (`self.CurrentStepIndex`) (+ (`self.PreviousStepIndex`) 1))
        (bind _output_3 (`|GetArrayItem` (`self.TowerStepArray`) _index_2))
        (if (`/Game/Blueprints/Actors/BP_TowerStep.IsActive` _output_3)
          (`/Game/Blueprints/Actors/BP_TowerStep.DestructStep` _output_3)
          (if (== (mod _index_2 (`self.StepsPerBlock`)) 0)
            (bind _output_4 (`|GetArrayItem` (`self.TowerPillarArray`) (/ _index_2 5)))
            (if (`/Game/Blueprints/Actors/BP_TowerPillar.isActive` _output_4)
              (`/Game/Blueprints/Actors/BP_TowerPillar.DestructPillar` _output_4)))))
      (set `self.PreviousStepIndex` (`self.CurrentStepIndex`))
      (`self.DestructTower`))))

(event `AddSteps`
  ;[0 0.02053 0.15 0.5] Spawning the stairs used in the tower at their designated location and rotation and adding them to an array
  (for _index (range 1 (+ (`SplineComponent.GetNumberOfSplinePoints` (`self.StepSpline`)) 1))
    (bind (_returnvalue_location _returnvalue_rotation) (`KismetMathLibrary.BreakTransform` (`SplineComponent.GetTransformAtSplinePoint` (`self.StepSpline`) _index "World" false)))
    (bind _returnvalue (`|SpawnActorFromClass` "/Game/Blueprints/Actors/BP_TowerStep.BP_TowerStep_C" (`KismetMathLibrary.MakeTransform` _returnvalue_location _returnvalue_rotation) "Undefined" "MultiplyWithRoot" null null))
    (`KismetArrayLibrary.Array_Add` (`self.TowerStepArray`) _returnvalue))
  (set `self.SafetyCollisionStartingPosition` (`SceneComponent.K2_GetComponentLocation` (`self.SafetyCapsuleCollider`)))
  (`self.SetSafetyCollision`))

(event `SetSafetyCollision`
  (bind _safetycapsulecollider (`self.SafetyCapsuleCollider`))
  (bind (_safetycollisionstartingposition_x _safetycollisionstartingposition_y _safetycollisionstartingposition_z) (`KismetMathLibrary.BreakVector` (`self.SafetyCollisionStartingPosition`)))
  ;[0.01235 0.15 0 0.5] Move safety collision up- and down as the tower is created
  (`SceneComponent.K2_SetWorldLocation` _safetycapsulecollider (`KismetMathLibrary.MakeVector` _safetycollisionstartingposition_x _safetycollisionstartingposition_y (+ _safetycollisionstartingposition_z (* (`self.PreviousStepIndex`) (`self.StepLocationOffset`)))) false true)
  (`KismetSystemLibrary.DrawDebugSphere` (`SceneComponent.K2_GetComponentLocation` (`self.SafetyCapsuleCollider`)) (`CapsuleComponent.CapsuleRadius` _safetycapsulecollider) 12 (struct :`R` 1.0 :`G` 1.0 :`B` 1.0 :`A` 1.0) 0.1))

(event `self.SafetyCapsuleCollider.OnComponentBeginOverlap`
  (params (OverlappedComponent :type "PrimitiveComponent Object Reference") (OtherActor :type "Actor Object Reference") (OtherComp :type "PrimitiveComponent Object Reference") (OtherBodyIndex :type Integer) (bFromSweep :type Boolean) (SweepResult :type "HitResult Structure (by ref)"))
  ;[0.000989 0.15 0 0.5] Check if something is blocking the construction site
  (`/Engine/EditorBlueprintResources/ActorMacros.Switch Has Authority`
    (:`Authority`
      (if (`KismetSystemLibrary.DoesImplementInterface` OtherActor "/Game/Blueprints/Interfaces/BPI_CharacterData.BPI_CharacterData_C")
        (`KismetSystemLibrary.PrintString` "Player Enter Collision")
        (set `self.PlayerBlocking` true)
        (else
          (`KismetSystemLibrary.PrintString` "something else is colliding"))))))

(event `self.SafetyCapsuleCollider.OnComponentEndOverlap`
  (params (OverlappedComponent :type "PrimitiveComponent Object Reference") (OtherActor :type "Actor Object Reference") (OtherComp :type "PrimitiveComponent Object Reference") (OtherBodyIndex :type Integer))
  ;[0.000989 0.15 0 0.5] Check if something is blocking the construction site
  (`/Engine/EditorBlueprintResources/ActorMacros.Switch Has Authority`
    (:`Authority`
      (if (`KismetSystemLibrary.DoesImplementInterface` OtherActor "/Game/Blueprints/Interfaces/BPI_CharacterData.BPI_CharacterData_C")
        (`KismetSystemLibrary.PrintString` "Player Exit Collision")
        (set `self.PlayerBlocking` false)
        (else
          (`KismetSystemLibrary.PrintString` "something else is colliding"))))))

(fn `FindEachStepLocation`
  (bind _returnvalue (`SceneComponent.K2_GetComponentToWorld` (`self.SM_ConstructionSite`)))
  (`SplineComponent.ClearSplinePoints` (`self.StepSpline`) true)
  (for _index (range (+ (`self.TowerStepsNeeded`) 1))
    (`SplineComponent.AddSplinePoint` (`self.StepSpline`) (`KismetMathLibrary.MakeVector` (.x (.location _returnvalue)) (.y (.location _returnvalue)) (+ (.z (.location _returnvalue)) (* _index (`self.StepLocationOffset`)))) "World" false)
    (`SplineComponent.SetRotationAtSplinePoint` (`self.StepSpline`) _index (`KismetMathLibrary.MakeRotator` 0.0 0.0 (+ (* _index (`self.StepRotationOffset`)) (.yaw (.rotation _returnvalue)))) "World" false))
  (`SplineComponent.UpdateSpline` (`self.StepSpline`))
  (`self.AddSteps`))

(fn `FindPointCloserToSplineEnd`
  (params (DistanceIncrement :type "Float (double-precision)"))
  (returns (PointCloserToSplineEnd :type "Vector Structure"))
  (return (+ (`SplineComponent.GetLocationAtSplinePoint` (`self.TowerSpline`) 0 "World") (* (`self.GetSplineDirection`) DistanceIncrement))))

(fn `FindTowerTop`
  (bind _sm_constructionsite (`self.SM_ConstructionSite`))
  (bind _returnvalue (`SceneComponent.K2_GetComponentLocation` _sm_constructionsite))
  (bind _outhit (`KismetSystemLibrary.LineTraceSingle` :`Start` _returnvalue :`End` (+ _returnvalue (* (`SceneComponent.GetUpVector` _sm_constructionsite) (`self.TowerTraceDistance`))) :`TraceChannel` "TraceTypeQuery1" :`DrawDebugType` "ForDuration"))
  (if (`GameplayStatics.BreakHitResult` _outhit)
    (bind _output_get (set `self.TowerTopPoint` (`KismetMathLibrary.MakeVector` (.x (`.Location` (`GameplayStatics.BreakHitResult` _outhit))) (.y (`.Location` (`GameplayStatics.BreakHitResult` _outhit))) (- (.z (`.Location` (`GameplayStatics.BreakHitResult` _outhit))) (`self.VerticalOffsetFromBlock`)))))
    (`KismetSystemLibrary.DrawDebugSphere` _output_get 25.0 12 (struct :`G` 0.180558 :`B` 1.0 :`A` 1.0) 5.0)
    (set `self.TowerDesiredHeight` (`KismetMathLibrary.Vector_Distance` (`SceneComponent.K2_GetComponentLocation` (`self.SM_ConstructionSite`)) _output_get))
    (else
      (bind _output_get_2 (set `self.TowerTopPoint` (`.TraceEnd` (`GameplayStatics.BreakHitResult` _outhit))))
      (`KismetSystemLibrary.DrawDebugSphere` _output_get_2 25.0 12 (struct :`R` 0.117571 :`G` 1.0 :`A` 1.0) 5.0)
      (set `self.TowerDesiredHeight` (`KismetMathLibrary.Vector_Distance` (`SceneComponent.K2_GetComponentLocation` (`self.SM_ConstructionSite`)) _output_get_2)))))

(fn `GetSplineDirection`
  (returns (DirectionVector :type "Vector Structure"))
  (return (`KismetMathLibrary.Normal` (- (`SplineComponent.GetLocationAtSplinePoint` (`self.TowerSpline`) 1 "World") (`SplineComponent.GetLocationAtSplinePoint` (`self.TowerSpline`) 0 "World")))))

(fn `GetStepsRequired`
  (bind _output_get (set `self.TowerBlocksNeeded` (`KismetMathLibrary.Round` (/ (`self.TowerDesiredHeight`) (`self.TowerBlockHeight`)))))
  (set `self.TowerStepsNeeded` (- (* _output_get (`self.StepsPerBlock`)) 1))
  (return))

(fn `Interact`
  (params (PlayerState :type "PlayerState Object Reference") (PlayerController :type "PlayerController Object Reference") (CharacterType :type "/Game/Blueprints/Enums/E_CharacterType Enum" :default "NewEnumerator2") (InteractInProgress :type Boolean))
  (returns (Success :type Boolean))
  (`/Engine/EditorBlueprintResources/ActorMacros.Switch Has Authority`
    (:`Authority`
      (if (`|EnumEquality` CharacterType "NewEnumerator1")
        (bind _output_get (set `self.InteractInProgress` InteractInProgress))
        (if _output_get
          (return true)
          (else
            (return false)))
        (else
          (set `self.InteractInProgress` false)
          (return false))))
    (:`Remote`
      (`KismetSystemLibrary.PrintString` "Does not have authority"))))

(fn `OnRep_InteractInProgress`
  (if (`self.InteractInProgress`)
    (`self.ConstructTower`)
    (else
      (`self.DestructTower`))))

(fn `UserConstructionScript`)