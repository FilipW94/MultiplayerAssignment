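; Bridge receiver actor that lays out a straight bridge at BeginPlay and tracks a hold-to-activate interaction from one character type.
; A forward line trace sets the end point, then a spline is filled at fixed step intervals and a BP_BridgeStep spawns at each point.
; Interact enables Tick on demand to raise or decay HoldDuration, disabling it at zero.
; The hold value does not yet drive the steps, and debug draws and prints remain.
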(event `self.ReceiveBeginPlay`
  (`SplineComponent.ClearSplinePoints` (`self.Spline`) true)
  (`self.FindBridgeEnd`)
  (`self.CreateSplineOpposites`))

(event `self.ReceiveTick`
  (params (DeltaSeconds :type "Float (single-precision)"))
  (if (`self.InteractInProgress`)
    ; Increase HoldDuration if Interacted with
    (set `self.HoldDuration` (+ (`self.HoldDuration`) DeltaSeconds))
    (elif (<= (`self.HoldDuration`) 0.0)
      ; Disable Tick if HoldDuration is reduced to 0
      (bind _output_get (set `self.HoldDuration` 0.0))
      (`KismetSystemLibrary.PrintString` (`KismetStringLibrary.Conv_DoubleToString` _output_get) true true (struct :`G` 0.66 :`B` 1.0 :`A` 1.0) 0.1)
      (`self.SetActorTickEnabled` false)
      (else
        ; Decrease HoldDuration if not Interacted with
        (bind _output_get_2 (set `self.HoldDuration` (- (`self.HoldDuration`) DeltaSeconds)))
        (`KismetSystemLibrary.PrintString` (`KismetStringLibrary.Conv_DoubleToString` _output_get_2) true true (struct :`G` 0.66 :`B` 1.0 :`A` 1.0) 0.1)))))

(event `CreateSplineOpposites`
  (`SplineComponent.AddSplinePoint` (`self.Spline`) (`SceneComponent.K2_GetComponentLocation` (`self.ReceiverCenter`)) "World" true)
  (`SplineComponent.AddSplinePoint` (`self.Spline`) (`self.BridgeEndPoint`) "World" true)
  (`self.FillSpline`))

(event `FillSpline`
  (`self.GetStepRequired`)
  (for _index (range (+ (`self.StepsNeeded`) 1))
    (bind _pointclosertosplineend (`self.FindPointCloserToSplineEnd` (* _index (`self.BridgeStepDistance`))))
    (`KismetSystemLibrary.DrawDebugSphere` _pointclosertosplineend 25.0 12 (struct :`R` 1.0 :`G` 1.0 :`B` 1.0 :`A` 1.0) 5.0)
    (`SplineComponent.AddSplinePoint` (`self.Spline`) _pointclosertosplineend "World" false))
  (`SplineComponent.RemoveSplinePoint` (`self.Spline`) 1 true)
  (`self.AddSteps`))

(event `AddSteps`
  (`KismetSystemLibrary.PrintString` (`KismetStringLibrary.Conv_IntToString` (`SplineComponent.GetNumberOfSplinePoints` (`self.Spline`))))
  (for _index (range (`SplineComponent.GetNumberOfSplinePoints` (`self.Spline`)))
    (bind (_returnvalue_location _returnvalue_rotation) (`KismetMathLibrary.BreakTransform` (`SplineComponent.GetTransformAtSplinePoint` (`self.Spline`) _index "World" false)))
    (bind _returnvalue (`|SpawnActorFromClass` "/Game/Blueprints/Actors/BP_BridgeStep.BP_BridgeStep_C" (`KismetMathLibrary.MakeTransform` _returnvalue_location _returnvalue_rotation) "Undefined" "MultiplyWithRoot" null null))
    (`KismetArrayLibrary.Array_Add` (`self.StepArray`) _returnvalue))
  (`KismetSystemLibrary.PrintString` (`KismetStringLibrary.Conv_DoubleToString` (/ (`self.HoldDuration`) (`KismetArrayLibrary.Array_Length` (`self.StepArray`))))))

(fn `FindBridgeEnd`
  (bind _receivercenter (`self.ReceiverCenter`))
  (bind _returnvalue (`SceneComponent.K2_GetComponentLocation` _receivercenter))
  (bind _outhit (`KismetSystemLibrary.LineTraceSingle` :`Start` _returnvalue :`End` (+ _returnvalue (* (`SceneComponent.GetForwardVector` _receivercenter) (`self.TraceDistance`))) :`TraceChannel` "TraceTypeQuery1" :`DrawDebugType` "ForDuration"))
  (if (`GameplayStatics.BreakHitResult` _outhit)
    (bind _output_get (set `self.BridgeEndPoint` (`.Location` (`GameplayStatics.BreakHitResult` _outhit))))
    (bind _output_get_2 (set `self.BridgeDesiredLength` (`KismetMathLibrary.Vector_Distance` (`SceneComponent.K2_GetComponentLocation` (`self.ReceiverCenter`)) _output_get)))
    (else
      (bind _output_get_3 (set `self.BridgeEndPoint` (`.TraceEnd` (`GameplayStatics.BreakHitResult` _outhit))))
      (set `self.BridgeDesiredLength` (`KismetMathLibrary.Vector_Distance` (`SceneComponent.K2_GetComponentLocation` (`self.ReceiverCenter`)) _output_get_3)))))

(fn `FindPointCloserToSplineEnd`
  (params (StepDistance :type "Float (double-precision)"))
  (returns (PointCloserToSplineEnd :type "Vector Structure"))
  (return (+ (`SplineComponent.GetLocationAtSplinePoint` (`self.Spline`) 0 "World") (* (`self.GetSplineDirection`) StepDistance))))

(fn `GetSplineDirection`
  (returns (DirectionVector :type "Vector Structure"))
  (return (`KismetMathLibrary.Normal` (- (`SplineComponent.GetLocationAtSplinePoint` (`self.Spline`) 1 "World") (`SplineComponent.GetLocationAtSplinePoint` (`self.Spline`) 0 "World")))))

(fn `GetStepRequired`
  (set `self.StepsNeeded` (`KismetMathLibrary.Round` (/ (`self.BridgeDesiredLength`) (`self.BridgeStepDistance`))))
  (return))

(fn `Interact`
  (params (PlayerState :type "PlayerState Object Reference") (CharacterType :type "/Game/Blueprints/Enums/E_CharacterType Enum" :default "NewEnumerator2") (InteractInProgress :type Boolean))
  (returns (Success :type Boolean))
  ; Make sure the correct character is interacting
  (if (`|EnumEquality` CharacterType "NewEnumerator0")
    (set `self.InteractInProgress` InteractInProgress)
    ; Tick handles both increase and decrease to HoldDuration but is disabled when not used so it needs to be enabled
    (if (`self.IsActorTickEnabled`)
      (if (>= (`self.HoldDuration`) (`self.RequiredHoldDuration`))
        (bind _output_get (set `self.HoldDuration` (`self.RequiredHoldDuration`)))
        (`KismetSystemLibrary.PrintString` (`KismetStringLibrary.Conv_DoubleToString` _output_get) true true (struct :`G` 0.66 :`B` 1.0 :`A` 1.0) 0.1)
        (return true)
        (else
          (`KismetSystemLibrary.PrintString` (`KismetStringLibrary.Conv_DoubleToString` (`self.HoldDuration`)) true true (struct :`G` 0.66 :`B` 1.0 :`A` 1.0) 0.1)
          (return false)))
      (else
        (`self.SetActorTickEnabled` true)))
    (else
      (set `self.InteractInProgress` false))))

(fn `UserConstructionScript`)