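; Spawn point actor that marks where a character type respawns, creating a PlayerStart at its SpawnLocation transform on BeginPlay.
; On authority, its trigger overlap reads the actor's type through BPI_CharacterData.
; If the type matches CharacterSpawn and this point is not already the closest spawn, it fires NewClosestSpawnDetected with itself to notify BP_RespawnHandler.
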(event `self.ReceiveBeginPlay`
  ; Spawn PlayerStart at assigned location
  (bind _returnvalue (`|SpawnActorFromClass` "/Script/Engine.PlayerStart" (`SceneComponent.K2_GetComponentToWorld` (`self.SpawnLocation`)) "Undefined" "MultiplyWithRoot" null null))
  (set `self.SpawnPoint` _returnvalue))

(event `self.UpdateSpawnPointTrigger.OnComponentBeginOverlap`
  (params (OverlappedComponent :type "PrimitiveComponent Object Reference") (OtherActor :type "Actor Object Reference") (OtherComp :type "PrimitiveComponent Object Reference") (OtherBodyIndex :type Integer) (bFromSweep :type Boolean) (SweepResult :type "HitResult Structure (by ref)"))
  ; Set new spawnpoint on overlap and tell the BP_RespawnHandler that this is the closest spawn for the corresponding character  type
  (`/Engine/EditorBlueprintResources/ActorMacros.Switch Has Authority`
    (:`Authority`
      (if (`KismetSystemLibrary.DoesImplementInterface` OtherActor "/Game/Blueprints/Interfaces/BPI_CharacterData.BPI_CharacterData_C")
        (bind _charactertype (message `/Game/Blueprints/Interfaces/BPI_CharacterData.GetCharacterData` OtherActor))
        (if (and (`|EnumEquality` _charactertype (`self.CharacterSpawn`)) (not (`self.ClosestSpawn`)))
          (`self.NewClosestSpawnDetected` self))))))

(fn `UserConstructionScript`)