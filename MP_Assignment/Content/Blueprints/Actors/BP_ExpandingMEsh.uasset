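; BP_ExpandingMEsh is an actor that fits its static mesh to the space between surfaces along one axis at BeginPlay.
; A forward visibility trace teleports the actor to the hit location, then triggers a second, backward trace.
; That trace's hit distance, divided by 100, sets the mesh's relative Y scale.
; Both traces draw debug lines, and the measured distance is printed to screen.
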(event `self.ReceiveBeginPlay`
  (`self.MoveCubeLineTrace`))

(fn `MoveCubeLineTrace`
  (bind _linetracestartingpoint (`self.LineTraceStartingPoint`))
  (bind _returnvalue (`SceneComponent.K2_GetComponentLocation` _linetracestartingpoint))
  (bind _outhit (`KismetSystemLibrary.LineTraceSingle` :`Start` _returnvalue :`End` (+ _returnvalue (* (`SceneComponent.GetForwardVector` _linetracestartingpoint) (`self.MoveCubeTraceDistance`))) :`TraceChannel` "TraceTypeQuery1" :`DrawDebugType` "ForDuration"))
  (if (`GameplayStatics.BreakHitResult` _outhit)
    (`self.K2_SetActorLocation` (`KismetMathLibrary.MakeVector` (.x (`.Location` (`GameplayStatics.BreakHitResult` _outhit))) (.y (`.Location` (`GameplayStatics.BreakHitResult` _outhit))) (.z (`.Location` (`GameplayStatics.BreakHitResult` _outhit)))) false true)
    (`self.ScaleLineTrace`)))

(fn `ScaleLineTrace`
  (bind _linetracestartingpoint (`self.LineTraceStartingPoint`))
  (bind _returnvalue (`SceneComponent.K2_GetComponentLocation` _linetracestartingpoint))
  (bind _outhit (`KismetSystemLibrary.LineTraceSingle` :`Start` _returnvalue :`End` (- _returnvalue (* (`SceneComponent.GetForwardVector` _linetracestartingpoint) (`self.ScaleTraceDistance`))) :`TraceChannel` "TraceTypeQuery1" :`DrawDebugType` "ForDuration"))
  (if (`GameplayStatics.BreakHitResult` _outhit)
    (`KismetSystemLibrary.PrintString` (`KismetStringLibrary.Conv_DoubleToString` (`.Distance` (`GameplayStatics.BreakHitResult` _outhit))))
    (`SceneComponent.SetRelativeScale3D` (`self.StaticMesh`) (`KismetMathLibrary.MakeVector` 1.0 (/ (`.Distance` (`GameplayStatics.BreakHitResult` _outhit)) 100.0) 1.0))))

(fn `UserConstructionScript`)