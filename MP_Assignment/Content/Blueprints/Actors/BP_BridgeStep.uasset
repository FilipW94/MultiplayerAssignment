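; A bridge step actor that assembles itself into its placed transform and can disintegrate again on demand.
; On BeginPlay it creates a dynamic material, hides the mesh via Disint_Amount, disables collision and picks a random offset spawn location and rotation.
; ConstructStep plays a timeline that lerps the dissolve and transform into place, enabling collision when finished.
; DestructStep disables collision and reverses the same timeline.
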(event `self.ReceiveBeginPlay`
  (bind _sm_bridgestep (`self.SM_BridgeStep`))
  (bind _returnvalue (`PrimitiveComponent.CreateDynamicMaterialInstance` _sm_bridgestep 0 (`PrimitiveComponent.GetMaterial` _sm_bridgestep 0) "None"))
  (bind _output_get (set `self.DisintMaterial` _returnvalue))
  (`/Engine/EditorBlueprintResources/StandardMacros.IsValid` _output_get
    (:`Is Valid`
      (`MaterialInstanceDynamic.SetScalarParameterValue` (`self.DisintMaterial`) "Disint_Amount" 1.0)
      (`PrimitiveComponent.SetCollisionEnabled` (`self.SM_BridgeStep`) "NoCollision")
      (set `self.TargetTransform` (`self.GetTransform`))
      (`self.FindRandomSpawnOffset`))
    (:`Is Not Valid`
      (`KismetSystemLibrary.PrintString` "Hello"))))

(event `ConstructStep`
  (bind _disintmaterial (`self.DisintMaterial`))
  (bind (_targettransform_location _targettransform_rotation) (`KismetMathLibrary.BreakTransform` (`self.TargetTransform`)))
  (bind (_direction _alpha) (`Timeline|TL_AlterMaterial` :!label _label)
    (:`Update`
      (`/Engine/EditorBlueprintResources/StandardMacros.IsValid` _disintmaterial
        (:`Is Valid`
          (`MaterialInstanceDynamic.SetScalarParameterValue` _disintmaterial "Disint_Amount" (`KismetMathLibrary.Lerp` 1.0 0.0 _alpha))
          (`self.K2_SetActorLocationAndRotation` (`KismetMathLibrary.VLerp` (`self.SpawnLocation`) _targettransform_location _alpha) (`KismetMathLibrary.RLerp` (`self.SpawnRotation`) _targettransform_rotation _alpha true)))
        (:`Is Not Valid`
          (`KismetSystemLibrary.PrintString` "Hello"))))
    (:`Finished`
      (switch `ETimelineDirection` _direction
        (:`Forward`
          (`PrimitiveComponent.SetCollisionEnabled` (`self.SM_BridgeStep`) "QueryAndPhysics"))))))

(event `DestructStep`
  (`PrimitiveComponent.SetCollisionEnabled` (`self.SM_BridgeStep`) "NoCollision")
  (goto _label :!via `Reverse`))

(fn `FindRandomSpawnOffset`
  (bind _returnvalue (`KismetMathLibrary.RandomFloatInRange` -150.0 150.0))
  (bind _returnvalue_2 (`KismetMathLibrary.RandomFloatInRange` -50.0 50.0))
  (bind _targettransform (`self.TargetTransform`))
  (set `self.SpawnLocation` (`KismetMathLibrary.MakeVector` (+ (.x (.location _targettransform)) _returnvalue) (+ (.y (.location _targettransform)) _returnvalue) (+ (.z (.location _targettransform)) _returnvalue)))
  (set `self.SpawnRotation` (`KismetMathLibrary.MakeRotator` (+ (.roll (.rotation _targettransform)) _returnvalue_2) (+ (.pitch (.rotation _targettransform)) _returnvalue_2) (+ (.yaw (.rotation _targettransform)) _returnvalue_2)))
  (return))

(fn `UserConstructionScript`)