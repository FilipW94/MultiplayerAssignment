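; BP_TowerStep is a tower step actor that materializes and dissolves on demand, starting invisible with collision disabled.
; ConstructStep plays a timeline that drives the RepNotify Alpha, whose OnRep lerps Disint_Amount on a dynamic material instance.
; Collision turns on only when construction finishes playing forward, while DestructStep disables it immediately and reverses the same timeline to dissolve the mesh.
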(event `self.ReceiveBeginPlay`
  (bind _sm_towerstep (`self.SM_TowerStep`))
  (bind _returnvalue (`PrimitiveComponent.CreateDynamicMaterialInstance` _sm_towerstep 0 (`PrimitiveComponent.GetMaterial` _sm_towerstep 0) "None"))
  (set `self.DisintMaterial` _returnvalue)
  (`PrimitiveComponent.SetCollisionEnabled` (`self.SM_TowerStep`) "NoCollision")
  (`MaterialInstanceDynamic.SetScalarParameterValue` (`self.DisintMaterial`) "Disint_Amount" 1.0))

(event `ConstructStep`
  (set `self.IsActive` true)
  (bind (_direction _alpha) (`Timeline|TL_Construct` :!label _label)
    (:`Update`
      (set `self.Alpha` _alpha))
    (:`Finished`
      (switch `ETimelineDirection` _direction
        (:`Forward`
          (`PrimitiveComponent.SetCollisionEnabled` (`self.SM_TowerStep`) "QueryAndPhysics"))))))

(event `DestructStep`
  (set `self.IsActive` false)
  (`PrimitiveComponent.SetCollisionEnabled` (`self.SM_TowerStep`) "NoCollision")
  (goto _label :!via `Reverse`))

(fn `OnRep_Alpha`
  (`MaterialInstanceDynamic.SetScalarParameterValue` (`self.DisintMaterial`) "Disint_Amount" (`KismetMathLibrary.Lerp` 1.0 0.0 (`self.Alpha`))))

(fn `UserConstructionScript`)