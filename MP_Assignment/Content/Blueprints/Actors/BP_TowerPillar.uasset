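; BP_TowerPillar is a pillar piece that materializes and dissolves on demand, starting invisible with collision off.
; BeginPlay creates a dynamic material instance and sets its Disint_Amount parameter to fully disintegrated.
; The Construct event plays a timeline that fades the pillar in, enabling collision and IsActive once it finishes forward.
; Destruct immediately disables both and reverses the same timeline to dissolve it.
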(event `self.ReceiveBeginPlay`
  (bind _sm_towerpillarpiece (`self.SM_TowerPillarPiece`))
  (`PrimitiveComponent.SetCollisionEnabled` (`self.SM_TowerPillarPiece`) "NoCollision")
  (bind _returnvalue (`PrimitiveComponent.CreateDynamicMaterialInstance` _sm_towerpillarpiece 0 (`PrimitiveComponent.GetMaterial` _sm_towerpillarpiece 0) "None"))
  (bind _output_get (set `self.DisintMaterial` _returnvalue))
  (`MaterialInstanceDynamic.SetScalarParameterValue` _output_get "Disint_Amount" 1.0))

(event `Construct`
  (bind (_direction _alpha) (`Timeline|TL_Construct` :!label _label)
    (:`Update`
      (`MaterialInstanceDynamic.SetScalarParameterValue` (`self.DisintMaterial`) "Disint_Amount" (`KismetMathLibrary.Lerp` 1.0 0.0 _alpha)))
    (:`Finished`
      (switch `ETimelineDirection` _direction
        (:`Forward`
          (`PrimitiveComponent.SetCollisionEnabled` (`self.SM_TowerPillarPiece`) "QueryAndPhysics")
          (set `self.isActive` true))))))

(event `Destruct`
  (`PrimitiveComponent.SetCollisionEnabled` (`self.SM_TowerPillarPiece`) "NoCollision")
  (set `self.isActive` false)
  (goto _label :!via `Reverse`))

(fn `UserConstructionScript`)