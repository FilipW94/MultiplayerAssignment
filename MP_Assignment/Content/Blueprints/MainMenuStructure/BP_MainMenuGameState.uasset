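; Main menu game state that keeps a list of joined player controllers and gives each a player index.
; Both a server-style event and a function add controllers and set their index, while a separate lookup finds a controller's position in PlayerArray.
; The replicated list prints its count on change, and Tick prints controller names on authority.
; Click handling is unfinished, with an empty WhoClicked and only debug prints in UpdateButton.
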(event `S_AddPlayerController`
  (params (Index :type Integer) (NewItem :type "PlayerController Object Reference (by ref)"))
  (`KismetArrayLibrary.Array_Add` (`self.PlayerControllers`) NewItem)
  (bind _asbp_main_menu_controller (cast `/Game/Blueprints/MainMenuStructure/BP_MainMenuController` NewItem))
  (set `/Game/Blueprints/MainMenuStructure/BP_MainMenuController.PlayerIndex` Index _asbp_main_menu_controller))

(event `WhoClicked`
  (params (NewParam :type "PlayerState Object Reference")))

(event `UpdateButton`
  (params (ClickerController :type "PlayerController Object Reference"))
  (`/Engine/EditorBlueprintResources/StandardMacros.IsValid` ClickerController
    (:`Is Valid`
      (bind _asbp_main_menu_controller (cast `/Game/Blueprints/MainMenuStructure/BP_MainMenuController` ClickerController)
        (:`CastFailed`
          (`KismetSystemLibrary.PrintString` "Hello"))))
    (:`Is Not Valid`
      (`KismetSystemLibrary.PrintString` "Hello"))))

(event `self.ReceiveTick`
  (params (DeltaSeconds :type "Float (single-precision)"))
  (for _array_element (`self.PlayerControllers`)
    (`/Engine/EditorBlueprintResources/ActorMacros.Switch Has Authority`
      (:`Authority`
        (`KismetSystemLibrary.PrintString` (`KismetSystemLibrary.GetDisplayName` _array_element))))))

(fn `AddPlayerController`
  (params (NewPlayerController :type "PlayerController Object Reference") (Index :type Integer))
  (bind _returnvalue (`KismetArrayLibrary.Array_Add` (`self.PlayerControllers`) NewPlayerController))
  (bind _asbp_main_menu_controller (cast `/Game/Blueprints/MainMenuStructure/BP_MainMenuController` NewPlayerController))
  (set `/Game/Blueprints/MainMenuStructure/BP_MainMenuController.PlayerIndex` _returnvalue _asbp_main_menu_controller))

(fn `GetPlayerControllerIndex`
  (params (Controller :type "/Game/Blueprints/MainMenuStructure/BP_MainMenuController Object Reference"))
  (returns (ControllerIndex :type Integer))
  (return (`KismetArrayLibrary.Array_Find` (`self.PlayerArray`) (`Controller.PlayerState` Controller))))

(fn `OnRep_PlayerControllers`
  (`KismetSystemLibrary.PrintString` (`KismetStringLibrary.Conv_IntToString` (`KismetArrayLibrary.Array_Length` (`self.PlayerControllers`)))))

(fn `UserConstructionScript`)