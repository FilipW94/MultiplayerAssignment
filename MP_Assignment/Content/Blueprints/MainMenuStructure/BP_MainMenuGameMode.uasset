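; BP_MainMenuGameMode is the main menu game mode that spawns a BP_MenuPawn for the first two players as they join.
; On PostLogin it matches the new player to controller 0 or 1, spawns a pawn indexed by PlayerNumber and increments that counter.
; Controller 0 possesses its new pawn, while controller 1's Possess call has no pawn connected.
; Any other player only triggers a debug print.
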(event `self.K2_PostLogin`
  (params (NewPlayer :type "PlayerController Object Reference"))
  (if (== NewPlayer (`GameplayStatics.GetPlayerController` 0))
    (bind _returnvalue (`|SpawnActorFromClass` "/Game/Blueprints/MainMenuStructure/BP_MenuPawn.BP_MenuPawn_C" (`KismetMathLibrary.MakeTransform` (0.0 0.0 0.0)) "Undefined" "MultiplyWithRoot" null (`self.PlayerNumber`) null))
    (`Controller.Possess` (`GameplayStatics.GetPlayerController` 0) _returnvalue)
    (bind _result (`/Engine/EditorBlueprintResources/StandardMacros.IncrementInt` (`self.PlayerNumber`))
      (:`  `
        (set `self.PlayerNumber` _result)))
    (elif (== NewPlayer (`GameplayStatics.GetPlayerController` 1))
      (`|SpawnActorFromClass` "/Game/Blueprints/MainMenuStructure/BP_MenuPawn.BP_MenuPawn_C" (`KismetMathLibrary.MakeTransform` (0.0 0.0 0.0)) "Undefined" "MultiplyWithRoot" null (`self.PlayerNumber`) null)
      (`Controller.Possess` (`GameplayStatics.GetPlayerController` 1) null)
      (bind _result_2 (`/Engine/EditorBlueprintResources/StandardMacros.IncrementInt` (`self.PlayerNumber`))
        (:`  `
          (set `self.PlayerNumber` _result_2)))
      (else
        (`KismetSystemLibrary.PrintString` "Hello")))))

(fn `UserConstructionScript`)