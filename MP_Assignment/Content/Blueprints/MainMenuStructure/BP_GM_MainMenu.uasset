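; Main menu game mode that registers up to two local players as they log in.
; PostLogin matches the new controller against player controller 0 or 1, casts it to BP_PC_MainMenu and stores it as Player1 or Player2.
; Each registered controller receives a PlayerIndex from the running PlayerAmount counter.
; SwapCharacter and EveryoneUpdate events are declared but empty.
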(event `self.K2_PostLogin`
  (params (NewPlayer :type "PlayerController Object Reference"))
  (bind _returnvalue (`GameplayStatics.GetPlayerController` 1))
  (bind _returnvalue_2 (`GameplayStatics.GetPlayerController` 0))
  (if (== NewPlayer _returnvalue_2)
    (bind _asbp_pc_main_menu (cast `/Game/Blueprints/MainMenuStructure/BP_PC_MainMenu` _returnvalue_2))
    (bind _output_get (set `self.Player1` _asbp_pc_main_menu))
    (set `/Game/Blueprints/MainMenuStructure/BP_PC_MainMenu.PlayerIndex` (`self.PlayerAmount`) _output_get)
    (bind _result (`/Engine/EditorBlueprintResources/StandardMacros.IncrementInt` (`self.PlayerAmount`))
      (:`  `
        (set `self.PlayerAmount` _result)))
    (elif (== NewPlayer _returnvalue)
      (bind _asbp_pc_main_menu_2 (cast `/Game/Blueprints/MainMenuStructure/BP_PC_MainMenu` _returnvalue))
      (bind _output_get_2 (set `self.Player2` _asbp_pc_main_menu_2))
      (set `/Game/Blueprints/MainMenuStructure/BP_PC_MainMenu.PlayerIndex` (`self.PlayerAmount`) _output_get_2)
      (bind _result_2 (`/Engine/EditorBlueprintResources/StandardMacros.IncrementInt` (`self.PlayerAmount`))
        (:`  `
          (set `self.PlayerAmount` _result_2))))))

(event `SwapCharacter`
  (params (PlayerController :type "PlayerController Object Reference") (CharacterType :type "/Game/Blueprints/Enums/E_CharacterType Enum" :default "NewEnumerator2")))

(event `EveryoneUpdate`)

(fn `UserConstructionScript`)