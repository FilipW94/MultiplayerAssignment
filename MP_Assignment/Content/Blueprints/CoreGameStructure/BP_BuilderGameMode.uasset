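; BP_BuilderGameMode is the game mode that assigns two players to the tower builder and bridge builder roles.
; On PostLogin it spawns and possesses BP_Char_TowerBuilder for controller 0 or BP_Char_BridgeBuilder for controller 1, counting players as it goes.
; Spawn tags are crossed: the tower builder uses the "BridgeBuilder" start and the bridge builder uses "TowerBuilder".
; Further players only trigger a debug message noting that a spectator class is needed.
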(event `self.K2_PostLogin`
  (params (NewPlayer :type "PlayerController Object Reference"))
  (bind _returnvalue (`GameplayStatics.GetPlayerController` 0))
  (bind _returnvalue_2 (`GameplayStatics.GetPlayerController` 1))
  (if (<= (`self.PlayersInGame`) 1)
    (if (== (`GameplayStatics.GetPlayerController` 0) NewPlayer)
      (bind _returnvalue_3 (`|SpawnActorFromClass` "/Game/ThirdPerson/Blueprints/BP_Char_TowerBuilder.BP_Char_TowerBuilder_C" (`self.GetTransform` (`self.K2_FindPlayerStart` _returnvalue "BridgeBuilder")) "Undefined" "MultiplyWithRoot" _returnvalue null))
      (`Controller.Possess` (`GameplayStatics.GetPlayerController` 0) _returnvalue_3)
      (bind _result (`/Engine/EditorBlueprintResources/StandardMacros.IncrementInt` (`self.PlayersInGame`))
        (:`  `
          (set `self.PlayersInGame` _result)))
      (elif (== (`GameplayStatics.GetPlayerController` 1) NewPlayer)
        (bind _returnvalue_4 (`|SpawnActorFromClass` "/Game/ThirdPerson/Blueprints/BP_Char_BridgeBuilder.BP_Char_BridgeBuilder_C" (`self.GetTransform` (`self.K2_FindPlayerStart` _returnvalue_2 "TowerBuilder")) "Undefined" "MultiplyWithRoot" _returnvalue_2 null))
        (`Controller.Possess` (`GameplayStatics.GetPlayerController` 1) _returnvalue_4)
        (bind _result_2 (`/Engine/EditorBlueprintResources/StandardMacros.IncrementInt` (`self.PlayersInGame`))
          (:`  `
            (set `self.PlayersInGame` _result_2)))
        (else
          (`KismetSystemLibrary.PrintString` "Not a valid controller"))))
    (else
      (`KismetSystemLibrary.PrintString` "need spectator class"))))

(fn `UserConstructionScript`)