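; Base HUD that creates and owns the player's main on-screen UI widget.
; On BeginPlay it adds WBP_BaseUI to the viewport and shows the character name from the owning pawn's character data, fetched through an interface message.
; It forwards construction zone status and interact prompt visibility to that widget through its own events.
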(event `self.ReceiveBeginPlay`
  (`self.AssignWidget`))

(event `AssignWidget`
  (bind _returnvalue (`|CreateWidget` "/Game/Widgets/WBP_BaseUI.WBP_BaseUI_C" (`self.GetOwningPlayerController`)))
  (bind _output_get (set `self.BaseUiRef` _returnvalue))
  (`UserWidget.AddToViewport` _output_get 0)
  (bind _charactertype (message `/Game/Blueprints/Interfaces/BPI_CharacterData.GetCharacterData` (`self.GetOwningPawn`)))
  (`/Game/Widgets/WBP_BaseUI.DisplayCharacterName` _output_get _charactertype))

(event `/Game/Blueprints/Interfaces/BPI_HUDCommunication.SetConstructionZoneStatus`
  (params (NewConstructionStatus :type Boolean))
  (`/Game/Widgets/WBP_BaseUI.SetConstructionZoneStatus` (`self.BaseUiRef`) NewConstructionStatus))

(event `/Game/Blueprints/Interfaces/BPI_HUDCommunication.SetInteractPrompt`
  (params (ShowPrompt :type Boolean))
  (`/Game/Widgets/WBP_BaseUI.ToggleInteractPrompt` (`self.BaseUiRef`) ShowPrompt))

(fn `UserConstructionScript`)