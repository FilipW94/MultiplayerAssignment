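; BP_BuilderController is a controller that handles interaction requests for its controlled pawn.
; Server_Interact runs on authority, asks the target for an interact message using the character, player state and progress, then passes it to the pawn's InteractStateCheck.
; GetPawnRef returns stored PawnRef when the controlled pawn is valid, attempting the BP_ThirdPersonCharacter cast and assignment only when it is invalid.
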(event `Server_Interact`
  (params (Character :type "/Game/Blueprints/Enums/E_CharacterType Enum" :default "NewEnumerator2") (PlayerState :type "PlayerState Object Reference") (InteractTarget :type "Actor Object Reference") (InteractInProgress :type Boolean))
  (bind _basepawnref (`self.GetPawnRef`))
  (`/Engine/EditorBlueprintResources/ActorMacros.Switch Has Authority`
    (:`Authority`
      (bind _success (message `/Game/Blueprints/Interfaces/BPI_Interact.Interact` InteractTarget PlayerState null Character InteractInProgress))
      (`/Engine/EditorBlueprintResources/StandardMacros.IsValid` _basepawnref
        (:`Is Valid`
          (`/Game/ThirdPerson/Blueprints/BP_ThirdPersonCharacter.InteractStateCheck` _basepawnref _success))))))

(fn `GetPawnRef`
  (returns (BasePawnRef :type "/Game/ThirdPerson/Blueprints/BP_ThirdPersonCharacter Object Reference"))
  (bind _returnvalue (`self.K2_GetPawn`))
  (`/Engine/EditorBlueprintResources/StandardMacros.IsValid` _returnvalue
    (:`Is Valid`
      _)
    (:`Is Not Valid`
      (bind _asbp_third_person_character (cast `/Game/ThirdPerson/Blueprints/BP_ThirdPersonCharacter` _returnvalue))
      (set `self.PawnRef` _asbp_third_person_character)))
  (return (`self.PawnRef`)))

(fn `UserConstructionScript`)