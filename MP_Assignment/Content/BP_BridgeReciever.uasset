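; BP_BridgeReciever is a hold-to-interact bridge receiver, apparently unfinished, that only one character type's player can complete.
; Interact wakes Tick, which builds HoldDuration while held, drains it on release and disables itself at zero.
; Interact returns true once the required hold is reached, printing progress for debugging.
; The spline is cleared at BeginPlay but never built, and FindBridgeEnd only runs a debug forward trace with its result unused.
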(event `self.ReceiveBeginPlay`
  (`SplineComponent.ClearSplinePoints` (`self.Spline`) true))

(event `self.ReceiveTick`
  (params (DeltaSeconds :type "Float (single-precision)"))
  (if (`self.InteractInProgress`)
    (set `self.HoldDuration` (+ (`self.HoldDuration`) DeltaSeconds))
    (elif (<= (`self.HoldDuration`) 0.0)
      (bind _output_get (set `self.HoldDuration` 0.0))
      (`KismetSystemLibrary.PrintString` (`KismetStringLibrary.Conv_DoubleToString` _output_get) true true (struct :`G` 0.66 :`B` 1.0 :`A` 1.0) 0.1)
      (`self.SetActorTickEnabled` false)
      (else
        (bind _output_get_2 (set `self.HoldDuration` (- (`self.HoldDuration`) DeltaSeconds)))
        (`KismetSystemLibrary.PrintString` (`KismetStringLibrary.Conv_DoubleToString` _output_get_2) true true (struct :`G` 0.66 :`B` 1.0 :`A` 1.0) 0.1)))))

(fn `FindBridgeEnd`
  (bind _receivercenter (`self.ReceiverCenter`))
  (bind _returnvalue (`SceneComponent.K2_GetComponentLocation` _receivercenter))
  (`KismetSystemLibrary.LineTraceSingle` :`Start` _returnvalue :`End` (+ _returnvalue (* (`SceneComponent.GetForwardVector` _receivercenter) (`self.TraceDistance`))) :`TraceChannel` "TraceTypeQuery1" :`DrawDebugType` "ForDuration"))

(fn `Interact`
  (params (PlayerState :type "PlayerState Object Reference") (InteractHoldDuration :type "Float (double-precision)") (CharacterType :type "/Game/E_CharacterType Enum" :default "NewEnumerator2") (InteractInProgress :type Boolean))
  (returns (Success :type Boolean))
  (set `self.InteractInProgress` InteractInProgress)
  (if (`self.IsActorTickEnabled`)
    (if InteractInProgress
      (if (and (== PlayerState (`/Game/BPFL_HelperFunctions.GetPlayerStateFromCharacterType` "NewEnumerator0")) (`self.InteractInProgress`))
        (if (>= (`self.HoldDuration`) (`self.RequiredHoldDuration`))
          (bind _output_get (set `self.HoldDuration` (`self.RequiredHoldDuration`)))
          (`KismetSystemLibrary.PrintString` (`KismetStringLibrary.Conv_DoubleToString` _output_get) true true (struct :`G` 0.66 :`B` 1.0 :`A` 1.0) 0.1)
          (return true)
          (else
            (`KismetSystemLibrary.PrintString` (`KismetStringLibrary.Conv_DoubleToString` (`self.HoldDuration`)) true true (struct :`G` 0.66 :`B` 1.0 :`A` 1.0) 0.1)
            (return false)))
        (else
          (set `self.InteractInProgress` false)
          (return false))))
    (else
      (`self.SetActorTickEnabled` true))))

(fn `UserConstructionScript`)